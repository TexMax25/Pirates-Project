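; BP_Character is a Character Blueprint that handles mouse look, movement, running and jumping.
; Movement axes follow only the control rotation's yaw, so looking up or down does not affect walking direction.
; Holding Running sets the IsRunning flag and raises max walk speed until release.
; Jump plays AM_Jump_Montage alongside the jump, and landing replays the montage from its JumpEnd section.
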(event `InputAxis|Turn Right / Left Mouse`
  (params (AxisValue :type "Float (single-precision)"))
  (`self.AddControllerYawInput` AxisValue))

(event `InputAxis|Move Forward / Backward`
  (params (AxisValue :type "Float (single-precision)"))
  (`self.AddMovementInput` (`KismetMathLibrary.GetForwardVector` (`KismetMathLibrary.MakeRotator` 0.0 0.0 (.yaw (`self.GetControlRotation`)))) AxisValue))

(event `InputAxis|Look Up / Down Mouse`
  (params (AxisValue :type "Float (single-precision)"))
  (`self.AddControllerPitchInput` AxisValue))

(event `InputAxis|Move Right / Left`
  (params (AxisValue :type "Float (single-precision)"))
  (`self.AddMovementInput` (`KismetMathLibrary.GetRightVector` (`KismetMathLibrary.MakeRotator` 0.0 0.0 (.yaw (`self.GetControlRotation`)))) AxisValue))

(event `InputAction|Running`
  (params (Key :type "Key Structure"))
  (bind _charactermovement (`self.CharacterMovement`))
  ;[1 1 1] Running
  (:`Pressed`
    (set `self.isRunning` true)
    (set `CharacterMovementComponent.MaxWalkSpeed` 600.0 _charactermovement))
  (:`Released`
    (set `self.isRunning` false)
    (set `CharacterMovementComponent.MaxWalkSpeed` 300.0 _charactermovement)))

(event `InputAction|Jump`
  (params (Key :type "Key Structure"))
  (:`Pressed`
    (`self.Jump`)
    (`self.PlayAnimMontage` "/Game/Personajes/Animations/AM_Jump_Montage.AM_Jump_Montage")))

(event `self.OnLanded`
  (params (Hit :type "HitResult Structure (by ref)"))
  (`self.PlayAnimMontage` "/Game/Personajes/Animations/AM_Jump_Montage.AM_Jump_Montage" 1.0 "JumpEnd"))

(fn `UserConstructionScript`)